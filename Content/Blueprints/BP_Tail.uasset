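; BP_Tail is an actor that follows a target, homing in on the player by default.
; On BeginPlay it fills an unset Target with the first BP_Player found in the level.
; Each Tick it moves along the normalized direction to Target at Speed, scaled by delta time, without sweeping.
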(event `self.ReceiveBeginPlay`
  ;[1 1 1] 태어날 때 target변수가 None이라면 플레이어를 찾아서 목적지로 기억하고싶다.
  (`/Engine/EditorBlueprintResources/StandardMacros.IsValid` (`self.Target`)
    (:`Is Not Valid`
      (bind _returnvalue (`GameplayStatics.GetActorOfClass` "/Game/Blueprints/BP_Player.BP_Player_C"))
      (set `self.Target` _returnvalue))))

(event `self.ReceiveTick`
  (params (DeltaSeconds :type "Float (single-precision)"))
  (`self.K2_SetActorLocation` (+ (`self.K2_GetActorLocation`) (* (`KismetMathLibrary.Normal` (- (`self.K2_GetActorLocation` (`self.Target`)) (`self.K2_GetActorLocation`))) (`self.Speed`) (`GameplayStatics.GetWorldDeltaSeconds`)))))

(fn `UserConstructionScript`)