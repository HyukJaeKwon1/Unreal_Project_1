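; BP_Player is the player actor, moved along its own right and up axes.
; BeginPlay resets its rotation to zero.
; Each Tick combines the Horizontal and Vertical values into a normalized direction, then scales it by Speed and delta seconds (P = P0 + vt).
; SetActorLocation applies the result without sweep, so movement ignores blocking collision.
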(event `self.ReceiveBeginPlay`
  (`self.K2_SetActorRotation` (struct)))

(event `self.ReceiveTick`
  (params (DeltaSeconds :type "Float (single-precision)"))
  ;[1 1 1] 오른쪽으로 이동하고싶다. P = P0 + vt(다음위치 = 현재위치 + 속도(방향 * 크기) * 시간)
  (`self.K2_SetActorLocation` (+ (`self.K2_GetActorLocation`) (* (`KismetMathLibrary.Normal` (+ (* (`self.GetInputAxisValue`) (`self.GetActorRightVector`)) (* (`self.GetInputAxisValue`) (`self.GetActorUpVector`)))) (`self.Speed`) DeltaSeconds))))

(fn `UserConstructionScript`)